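; BP_Enemy is an enemy that chases the player and damages them on contact.
; Each tick it aligns its TopUI widget, issues an AI move toward the player, turns to face them and checks its Hp.
; Capsule overlap with the player subtracts Damage from the player's Hp and prints the result.
; At zero Hp or below, it resets the player's CurrentTarget and ClosestDistance, then destroys itself.
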(event OnComponentBeginOverlap(CapsuleComponent)
  (params (OverlappedComponent :type Primitive%20Component%20Object%20Reference) (OtherActor :type Actor%20Object%20Reference) (OtherComp :type Primitive%20Component%20Object%20Reference) (OtherBodyIndex :type Integer) (bFromSweep :type Boolean) (SweepResult :type Hit%20Result%20Structure%20%28by%20ref%29))
  (bind _returnvalue (Game|GetPlayerCharacter 0))
  ;[1 1 1] Overlap
  (if (== OtherActor _returnvalue)
    (bind _asbp_player_character (Utilities|Casting|CastToBP_PlayerCharacter _returnvalue))
    (Variables|/Game/Blueprints/BP_PlayerCharacter.BP_PlayerCharacter_C|SetHp _asbp_player_character (- (Variables|/Game/Blueprints/BP_PlayerCharacter.BP_PlayerCharacter_C|GetHp _asbp_player_character) (Variables|Default|GetDamage)))
    (Development|PrintString (Utilities|String|ToString(Float) (Variables|/Game/Blueprints/BP_PlayerCharacter.BP_PlayerCharacter_C|GetHp _asbp_player_character)))))

(event Custom|Die
  ;[1 1 1] Die and reset target
  (if (Variables|Default|GetDead?)
    (bind _outactors (Actor|GetAllActorsOfClass "/Game/Blueprints/BP_PlayerCharacter.BP_PlayerCharacter_C"))
    (Variables|/Game/Blueprints/BP_PlayerCharacter.BP_PlayerCharacter_C|SetCurrentTarget (Utilities|Array|Get(acopy) _outactors) (Variables|Default|GetEmptyActor))
    (Variables|/Game/Blueprints/BP_PlayerCharacter.BP_PlayerCharacter_C|SetClosestDistance (Utilities|Array|Get(acopy) _outactors) 9999.0)
    (Actor|DestroyActor self)))

(event EventBeginPlay
  (Rendering|SetCastShadow (Variables|Default|GetTopUI) false))

(event EventTick
  (params (DeltaSeconds :type Float%20%28single-precision%29))
  (bind _returnvalue (Game|GetPlayerCharacter 0))
  (bind _self self)
  ;[1 1 1] Event Tick
  (CallFunction|AlighWidgets (Variables|Default|GetTopUI) self)
  (AI|AIMoveTo _self "0, 0, 0" _returnvalue 5.0 false
    (:then
      (CallFunction|MakeCharacterFaceYou _self _returnvalue)
      (if (<= (Variables|Default|GetHp) 0.0)
        (Variables|Default|SetDead? true)
        (CallFunction|Die)
        (else
          (Variables|Default|SetDead? false))))))

(fn ConstructionScript)