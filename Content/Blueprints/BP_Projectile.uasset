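; BP_Projectile is a homing projectile that chases the player's current target and damages enemies.
; On BeginPlay it finds BP_PlayerCharacter and caches its CurrentTarget.
; Tick calls ChaseTarget, which, after a short Delay, points ProjectileMovement velocity at the target at fixed speed while it remains valid.
; Capsule overlap with a BP_Enemy subtracts the player's Damage from its Hp and destroys the projectile; other actors are ignored.
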(event OnComponentBeginOverlap(Capsule)
  (params (OverlappedComponent :type Primitive%20Component%20Object%20Reference) (OtherActor :type Actor%20Object%20Reference) (OtherComp :type Primitive%20Component%20Object%20Reference) (OtherBodyIndex :type Integer) (bFromSweep :type Boolean) (SweepResult :type Hit%20Result%20Structure%20%28by%20ref%29))
  ;[1 1 1] Overlap
  (bind _asbp_enemy (Utilities|Casting|CastToBP_Enemy OtherActor))
  (bind _outactors (Actor|GetAllActorsOfClass "/Game/Blueprints/BP_PlayerCharacter.BP_PlayerCharacter_C"))
  (if (== OtherActor _asbp_enemy)
    (Variables|/Game/Blueprints/BP_Enemy.BP_Enemy_C|SetHp _asbp_enemy (- (Variables|/Game/Blueprints/BP_Enemy.BP_Enemy_C|GetHp _asbp_enemy) (Variables|/Game/Blueprints/BP_PlayerCharacter.BP_PlayerCharacter_C|GetDamage (Utilities|Array|Get(acopy) _outactors))))
    (Development|PrintString "I have hit an enemy")
    (Actor|DestroyActor)
    (else
      (Actor|DestroyActor))))

(event Custom|ChaseTarget
  ;[1 1 1] ChaseTarget
  (Variables|Default|GetCurrent%20Target
    (:then
      (Utilities|FlowControl|Delay 0.05)
      (Variables|/Script/Engine.MovementComponent|SetVelocity (Variables|Default|GetProjectileMovement) (* (Math|Vector|Normalize (- (Transformation|GetActorLocation (Variables|Default|GetCurrent%20Target)) (Transformation|GetActorLocation))) 1500)))
    (:else)))

(event EventBeginPlay
  ;[1 1 1] BeginPlay
  (bind _outactors (Actor|GetAllActorsOfClass "/Game/Blueprints/BP_PlayerCharacter.BP_PlayerCharacter_C"))
  (Variables|Default|SetPlayerRef (Utilities|Array|Get(acopy) _outactors))
  (Variables|Default|SetCurrent%20Target (Variables|/Game/Blueprints/BP_PlayerCharacter.BP_PlayerCharacter_C|GetCurrentTarget (Utilities|Array|Get(acopy) _outactors))))

(event EventTick
  (params (DeltaSeconds :type Float%20%28single-precision%29))
  ;[1 1 1] Event Tick
  (CallFunction|ChaseTarget))

(fn ConstructionScript)