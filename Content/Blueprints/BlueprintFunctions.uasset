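; Blueprint function library with two helpers for orienting widgets and characters.
; AlighWidgets places a widget at a fixed world-space offset above and beside an actor, rotated toward player 0's camera with a look-at rotation.
; MakeCharacterFaceYou sets an actor's rotation from a look-at, but feeds the target's location as both start and end, so it does not actually compute a facing direction.
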(fn AlighWidgets
  (params (Widget :type Widget%20Component%20Object%20Reference) (Actor :type Actor%20Object%20Reference))
  (bind _rootcomponent (Variables|/Script/Engine.Actor|GetRootComponent Actor))
  (bind _returnvalue (Transformation|GetWorldLocation _rootcomponent))
  (Transformation|SetWorldLocationAndRotation Widget (Math|Vector|MakeVector (.x _returnvalue) (+ (.y _returnvalue) -35.0) (+ (.z _returnvalue) 135.0)) (Math|Rotator|FindLookatRotation (Transformation|GetWorldLocation Widget) (Transformation|GetWorldLocation (Variables|/Script/Engine.PlayerCameraManager|GetTransformComponent (Game|GetPlayerCameraManager 0)))) false false))

(fn MakeCharacterFaceYou
  (params (Sef :type Actor%20Object%20Reference) (Target :type Actor%20Object%20Reference))
  (Transformation|SetActorRotation Sef (Math|Rotator|FindLookatRotation (Transformation|GetWorldLocation (Variables|/Script/Engine.Actor|GetRootComponent Target)) (Transformation|GetWorldLocation (Variables|/Script/Engine.Actor|GetRootComponent Target)))))