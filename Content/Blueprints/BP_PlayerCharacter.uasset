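; BP_PlayerCharacter is the player character, which moves on input and fires projectiles automatically.
; MoveForward and MoveRight axis inputs add movement along the actor's forward and right vectors.
; On BeginPlay, a looping timer set by function name calls FireProjectile every half second, spawning a BP_Projectile at the actor's location facing the control rotation.
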(event Custom|FireProjectile
  (Game|SpawnActorfromClass "/Game/Blueprints/BP_Projectile.BP_Projectile_C" (Math|Transform|MakeTransform (Transformation|GetActorLocation) (Pawn|GetControlRotation :!class /Script/Engine.Pawn) "1.000000,1.000000,1.000000") "Undefined" "MultiplyWithRoot" 0 0))

(event EventBeginPlay
  (Utilities|Time|SetTimerbyFunctionName 0 "FireProjectile" 0.5 true))

(event Collision|EventActorBeginOverlap
  (params (OtherActor :type Actor%20Object%20Reference)))

(event EventTick
  (params (DeltaSeconds :type Float%20%28single-precision%29)))

(event Input|AxisEvents|InputAxisMoveForward
  (params (AxisValue :type Float%20%28single-precision%29))
  (Pawn|Input|AddMovementInput (Transformation|GetActorForwardVector) AxisValue false))

(event Input|AxisEvents|InputAxisMoveRight
  (params (AxisValue :type Float%20%28single-precision%29))
  (Pawn|Input|AddMovementInput (Transformation|GetActorRightVector) AxisValue false))

(fn ConstructionScript)